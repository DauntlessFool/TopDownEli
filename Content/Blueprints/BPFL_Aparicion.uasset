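; Blueprint function library for spawning ("Aparicion") that finds a random navigable position inside a given box component.
; ObtenerPosicionValida picks random points in the box's bounds and projects them onto the navmesh, up to Reintentos times.
; The returned location re-evaluates the random projection, so it can differ from the point that passed the check.
; An invalid box or exhausted retries returns failure with a zero vector.
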(fn ObtenerPosicionValida
  (params (Caja :type Box%20Component%20Object%20Reference) (Reintentos :type Integer))
  (bind _returnvalue (Transformation|GetWorldLocation Caja))
  (bind _returnvalue_2 (Components|Box|GetScaledBoxExtent Caja))
  (bind _returnvalue_3 (Math|Random|RandomPointinBoundingBox _returnvalue _returnvalue_2))
  (bind (_projectedlocation _returnvalue_4) (AI|Navigation|ProjectPointtoNavigation Caja _returnvalue_3 0 0 "200.000000,200.000000,500.000000"))
  (if (Utilities|IsValid Caja)
    (for _index (range 0 (- Reintentos 1))
      (if _returnvalue_4
        (return true _projectedlocation)))
    (return false "0, 0, 0")
    (else
      (return false "0, 0, 0"))))