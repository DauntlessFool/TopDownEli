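; BP_Projectile is a projectile fired toward a target point, carrying the owning Player's speed and damage.
; BeginPlay rotates it to face Target and caps ProjectileMovement speed at the Player's ProjectileSpeed.
; Overlapping a non-instigator actor with a BP_HealthComponent applies Player damage and destroys it, gated by a HasHit flag that other overlaps leave set.
; Tick also destroys it within a short distance of Target.
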(event EventBeginPlay
  (bind _projectilemovement (Variables|Default|GetProjectileMovement))
  (Utilities|IsValid (Variables|Default|GetPlayer)
    (:Is%20Valid
      (Transformation|SetActorRotation (Math|Rotator|FindLookatRotation (Transformation|GetActorLocation) (Variables|Default|GetTarget)))
      (Variables|/Script/Engine.ProjectileMovementComponent|SetInitialSpeed _projectilemovement 0.0)
      (Variables|/Script/Engine.ProjectileMovementComponent|SetMaxSpeed _projectilemovement (Variables|/Game/TopDown/Blueprints/BP_TopDownCharacter.BP_TopDownCharacter_C|GetProjectile%20Speed (Variables|Default|GetPlayer))))))

(event EventTick
  (params (DeltaSeconds :type Float%20%28single-precision%29))
  (if (<= (Math|Vector|Distance(Vector) (Transformation|GetActorLocation) (Variables|Default|GetTarget)) 2e+01)
    (Actor|DestroyActor)))

(event Collision|EventActorBeginOverlap
  (params (OtherActor :type Actor%20Object%20Reference))
  (bind _returnvalue (Actor|GetComponentbyClass OtherActor "/Game/Blueprints/Components/BP_HealthComponent.BP_HealthComponent_C"))
  (if (not (Variables|Default|GetHasHit))
    (Variables|Default|SetHasHit true)
    (if (!= OtherActor (Variables|Default|GetInstigatorActor))
      (if (Utilities|IsValid _returnvalue)
        (Default|RecibirDaño _returnvalue (Variables|/Game/TopDown/Blueprints/BP_TopDownCharacter.BP_TopDownCharacter_C|GetDmg (Variables|Default|GetPlayer)))
        (Variables|Default|SetHasHit false)
        (Actor|DestroyActor)))))

(fn ConstructionScript)