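; Health component that tracks current health against a maximum for the actor that owns it.
; RecibirDaño subtracts damage and Curacion adds healing, both clamping the result between zero and the maximum and broadcasting OnHealthChanged.
; Damage also prints the new health and component name for debugging, and fires the AlMorir dispatcher whenever health is at zero.
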(event EventBeginPlay)

(event EventTick
  (params (DeltaSeconds :type Float%20%28single-precision%29)))

(fn RecibirDaño
  (params (Cantidad :type Float%20%28double-precision%29))
  (bind _output_get (Variables|Default|SetVidaActual (Math|Float|Clamp(Float) (- (Variables|Default|GetVidaActual) Cantidad) 0.0 (Variables|Default|GetVidaMaxima))))
  (Development|PrintString (Utilities|String|ToString(Float) (Variables|Default|GetVidaActual)))
  (Development|PrintString (Utilities|GetDisplayName self))
  (Default|CallOnHealthChanged)
  (if (<= _output_get 0.0)
    (Default|CallAlMorir)))

(fn Curacion
  (params (Cantidad :type Float%20%28double-precision%29))
  (Variables|Default|SetVidaActual (Math|Float|Clamp(Float) (+ Cantidad (Variables|Default|GetVidaActual)) 0.0 (Variables|Default|GetVidaMaxima)))
  (Default|CallOnHealthChanged))